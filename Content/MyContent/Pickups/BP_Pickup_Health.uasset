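; Health pickup Blueprint that heals the character who collects it.
; It overrides Pickup to call HealHealth on that character.
; OnDeactivate and OnReactivate extend the parent's behavior by hiding and showing the two cone components.
; The event graph and construction script add no logic of their own.
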(event EventBeginPlay
  (|CallParentFunction) ; This node is disabled and will not be called.\nDrag off pins to build functionality.
)

(event Collision|EventActorBeginOverlap
  (params (OtherActor :type Actor%20Object%20Reference)))

(event EventTick
  (params (DeltaSeconds :type Float%20%28single-precision%29))
  (|CallParentFunction DeltaSeconds) ; This node is disabled and will not be called.\nDrag off pins to build functionality.
)

(fn ConstructionScript
  (|CallParentFunction))

(fn OnDeactivate
  (|CallParentFunction)
  (Rendering|SetVisibility (Variables|Default|GetCone) false false))

(fn OnReactivate
  (|CallParentFunction)
  (Rendering|SetVisibility (Variables|Default|GetCone) true false))

(fn Pickup
  (params (Character :type BP%20Character%20Object%20Reference))
  (Default|HealHealth Character))
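; GM_Lobby is the lobby game mode that spawns each joining player at a numbered Player Start.
; On PostLogin it loops over all Player Starts, using the current player state count minus one to choose which tag to match, from Player1 to Player4.
; It restarts the new player at the first matching start, so slots follow the player count at login rather than tracking which starts are occupied.
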(event EventPostLogin
  (params (NewPlayer :type Player%20Controller%20Object%20Reference))
  (bind _outactors (Actor|GetAllActorsOfClass "/Script/Engine.PlayerStart"))
  (bind _array_element (Utilities|Array|ForEachLoopwithBreak _outactors :!label _label)
    (:LoopBody
      (if (Utilities|Select :Index (- (Class|GameplayStatics|GetNumPlayerStates) 1) :Option%200 (== (Variables|/Script/Engine.PlayerStart|GetPlayerStartTag _array_element) "Player1") :Option%201 (== (Variables|/Script/Engine.PlayerStart|GetPlayerStartTag _array_element) "Player2") :Option%202 (== (Variables|/Script/Engine.PlayerStart|GetPlayerStartTag _array_element) "Player3") :Option%203 (== (Variables|/Script/Engine.PlayerStart|GetPlayerStartTag _array_element) "Player4"))
        (Class|GameModeBase|RestartPlayeratPlayerStart NewPlayer _array_element)
        (goto _label Break)))))

(fn ConstructionScript)
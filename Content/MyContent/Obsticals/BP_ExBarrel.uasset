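; Explosive barrel that detonates on its first point damage, launching itself along the shot direction; later hits only nudge it.
; ApplyDamage sphere-overlaps Pawn and Destructible actors within ExplosionRadius, line-traces for clear visibility, then deals point damage that falls off linearly with distance.
; A separate MultiEffects event activates and detaches the particle system and swaps the mesh to its exploded material.
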(event Custom|Multi_Effects
  (Components|Activation|Activate (Variables|Default|GetParticleSystem) false)
  (Transformation|DetachFromComponent (Variables|Default|GetParticleSystem) "KeepWorld" "KeepWorld" "KeepWorld" true)
  (Rendering|Material|SetMaterial (Variables|Default|GetBarrleMesh) 0 "/Game/Megascans/3D_Assets/Rusty_Metal_Barrel_teraccgda/MI_Rusty_Metal_Barrel_Exploded.MI_Rusty_Metal_Barrel_Exploded"))

(event Game|Damage|EventPointDamage
  (params (Damage :type Float%20%28single-precision%29) (DamageType :type Damage%20Type%20Object%20Reference) (HitLocation :type Vector :default "0, 0, 0") (HitNormal :type Vector :default "0, 0, 0") (HitComponent :type Primitive%20Component%20Object%20Reference) (BoneName :type Name :default "None") (ShotFromDirection :type Vector :default "0, 0, 0") (InstigatedBy :type Controller%20Object%20Reference) (DamageCauser :type Actor%20Object%20Reference) (HitInfo :type Hit%20Result%20Structure%20%28by%20ref%29))
  (if (not (Variables|Default|GetIsDestroyed))
    (Variables|Default|SetIsDestroyed true)
    (Physics|AddImpulse (Variables|Default|GetBarrleMesh) (* ShotFromDirection 2e+03) "None" true)
    (CallFunction|ApplyDamage)
    (Components|Activation|Activate (Variables|Default|GetParticleSystem) false)
    (Transformation|DetachFromComponent (Variables|Default|GetParticleSystem) "KeepWorld" "KeepWorld" "KeepWorld" true)
    (CallFunction|MultiEffects)
    (else
      (Physics|AddImpulse (Variables|Default|GetBarrleMesh) (* ShotFromDirection 1.5e+02) "None" true))))

(fn ConstructionScript)

(fn ApplyDamage
  (bind _explosionradius (Variables|Default|GetExplosionRadius))
  (bind _outactors (Collision|SphereOverlapActors (Transformation|GetWorldLocation _explosionradius) (Components|Sphere|GetScaledSphereRadius _explosionradius) (Utilities|Array|MakeArray "ObjectTypeQuery3" "ObjectTypeQuery6") 0 (Utilities|Array|MakeArray self)))
  (for _array_element _outactors
    (LocalVariables|SetLTestActor _array_element)
    (bind (_outhit _returnvalue) (Collision|LineTraceByChannel (Transformation|GetWorldLocation (Variables|Default|GetExplosionRadius)) (Transformation|GetActorLocation (LocalVariables|GetLTestActor)) "TraceTypeQuery1" false 0 "None"))
    (if _returnvalue
      (if (== (.HitActor (Collision|BreakHitResult _outhit)) (LocalVariables|GetLTestActor))
        (Game|Damage|ApplyPointDamage (LocalVariables|GetLTestActor) (* (Variables|Default|GetDamage) (- 1.0 (/ (.Distance (Collision|BreakHitResult _outhit)) (Components|Sphere|GetScaledSphereRadius (Variables|Default|GetExplosionRadius))))) (Math|Vector|GetForwardVector (Math|Rotator|FindLookatRotation (.TraceStart (Collision|BreakHitResult _outhit)) (.TraceEnd (Collision|BreakHitResult _outhit)))) _outhit 0 self)))))